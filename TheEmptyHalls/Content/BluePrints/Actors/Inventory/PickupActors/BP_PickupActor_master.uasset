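; Base pickup actor that lets an L1_Character collect an item into its inventory.
; Sphere overlap stores the overlapping actor and toggles that character's pickup prompt, using the item name from the Item class defaults.
; While overlapping, Interact adds the Item and Amount through the character's BPCInventory.
; On success it keeps any remainder as the new Amount, or destroys itself when none is left.
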(event `self.Sphere.OnComponentBeginOverlap`
  (params (OverlappedComponent :type "PrimitiveComponent Object Reference") (OtherActor :type "Actor Object Reference") (OtherComp :type "PrimitiveComponent Object Reference") (OtherBodyIndex :type Integer) (bFromSweep :type Boolean) (SweepResult :type "HitResult Structure (by ref)"))
  (bind _itemdata_itemname (break `/Game/BluePrints/Structs/S_ItemData` (defaults `Object` (`self.Item`))))
  (set `self.IsOverlapping` true)
  (bind _output_get (set `self.Other Actor` OtherActor))
  (bind _asl1_character (cast `/Game/Game_BP/Level1/L1_Character` _output_get))
  (`/Game/Game_BP/Level1/L1_Character.PickupWidgetToggle` _asl1_character (`KismetTextLibrary.Conv_StringToText` (`KismetStringLibrary.Conv_NameToString` _itemdata_itemname)) (`self.IsOverlapping`) null))

(event `self.Sphere.OnComponentEndOverlap`
  (params (OverlappedComponent :type "PrimitiveComponent Object Reference") (OtherActor :type "Actor Object Reference") (OtherComp :type "PrimitiveComponent Object Reference") (OtherBodyIndex :type Integer))
  (set `self.IsOverlapping` false)
  (bind _output_get (set `self.Other Actor` OtherActor))
  (bind _asl1_character (cast `/Game/Game_BP/Level1/L1_Character` _output_get))
  (`/Game/Game_BP/Level1/L1_Character.PickupWidgetToggle` _asl1_character "item" (`self.IsOverlapping`) _output_get))

(event `/Game/BluePrints/Interfaces/BPI_Interaction.Interact`
  (if (`self.IsOverlapping`)
    (bind _asl1_character (cast `/Game/Game_BP/Level1/L1_Character` (`self.Other Actor`)))
    (bind (_succes_ _remainder) (`/Game/BluePrints/BlueprintComponents/BPC_Inventory.add Item` (`/Game/Game_BP/Level1/L1_Character.BPC_Inventory` _asl1_character) (`self.Item`) (`self.Amount`)))
    (if _succes_
      (if (> _remainder 0)
        (set `self.Amount` _remainder)
        (else
          (`self.K2_DestroyActor`))))))

(fn `UserConstructionScript`)